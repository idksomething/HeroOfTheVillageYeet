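; Player character Blueprint with a three-hit sword combo, health and death handling.
; Left mouse cycles three attack montages through a combo counter with save and reset events, and SwordBox hits apply SwordDamageBP damage.
; BeginPlay adds a health bar widget; any damage lowers health, while every actor overlap subtracts a fixed amount.
; Only the overlap path checks for death, which blocks movement, plays a death animation and reloads LevelCave after a delay.
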(event OnComponentHit(swordBox)
  (params (HitComponent :type Primitive%20Component%20Object%20Reference) (OtherActor :type Actor%20Object%20Reference) (OtherComp :type Primitive%20Component%20Object%20Reference) (NormalImpulse :type Vector :default "0, 0, 0") (Hit :type Hit%20Result%20Structure%20%28by%20ref%29))
  ;[1 1 1] Applys damage and uses tha damage class i created to decide how much damage it does.
  (Game|Damage|ApplyDamage OtherActor 1.0 0 0 "/Game/Blueprints/SwordDamageBP.SwordDamageBP_C")
  (Development|PrintString (Utilities|GetObjectName OtherActor)))

(event Custom|ResetCombo
  ;[1 1 1] Resets and saves combo for the attack
  (Variables|Default|SetComboCounter 0)
  (Variables|Default|SetSaveAttack false)
  (Variables|Default|SetIsAttacking false))

(event Custom|SaveComboAttack
  ;[1 1 1] Resets and saves combo for the attack
  (if (Variables|Default|GetSaveAttack)
    (Variables|Default|SetSaveAttack false)))

(event EventBeginPlay
  ;[1 1 1] When the game start the healthbar is there.
  (bind _returnvalue (UserInterface|CreateWidget "/Game/HealthBar.HealthBar_C"))
  (bind _output_get (Variables|Default|SetReferenceToHealthBar _returnvalue))
  (UserInterface|Viewport|AddtoViewport _output_get 0))

(event Collision|EventActorBeginOverlap
  (params (OtherActor :type Actor%20Object%20Reference))
  ;[1 1 1] Sets if your health drops to zero or less you die and respawn at the start of the level.
  (bind _output_get (Variables|Default|SetCurrentHealth (- (Variables|Default|GetCurrentHealth) 1e+02)))
  (Math|Float|CompareFloat _output_get 0.0
    (:==
      _)
    (:<
      _))
  (Input|SetIgnoreMoveInput (Game|GetPlayerController 0) true)
  (Components|Animation|PlayAnimation (Variables|Character|GetMesh) "/Game/Frank_RPG_Sword1/Animations/Preview_Character/45_Frank_RPG_Sword_Die_01.45_Frank_RPG_Sword_Die_01" false)
  (Utilities|FlowControl|Delay 3.0)
  (Game|OpenLevel(byName) "LevelCave"))

(event Game|Damage|EventAnyDamage
  (params (Damage :type Float%20%28single-precision%29) (DamageType :type Damage%20Type%20Object%20Reference) (InstigatedBy :type Controller%20Object%20Reference) (DamageCauser :type Actor%20Object%20Reference))
  (Variables|Default|SetCurrentHealth (- (Variables|Default|GetCurrentHealth) Damage)))

(event Input|MouseEvents|LeftMouseButton
  (params (Key :type Key%20Structure))
  (bind _mesh (Variables|Character|GetMesh))
  (bind _returnvalue (Components|SkeletalMesh|GetAnimInstance _mesh))
  ;[1 1 1] Makes the combo animation when you click the left mouse button.
  (:Pressed
    (if (Variables|Default|GetIsAttacking)
      (Variables|Default|SetIsAttacking true)
      (else
        (Variables|Default|SetSaveAttack true)
        (switch int (Variables|Default|GetComboCounter)
          (:0
            (Variables|Default|SetComboCounter 1)
            (Animation|Montage|MontagePlay _returnvalue "/Game/AttackCombo/AnimMontage1.AnimMontage1" 1.0 "MontageLength" 0.0 true))
          (:1
            (Variables|Default|SetComboCounter 2)
            (Animation|Montage|MontagePlay _returnvalue "/Game/AttackCombo/AnimMontage2.AnimMontage2" 1.0 "MontageLength" 0.0 true))
          (:2
            (Variables|Default|SetComboCounter 0)
            (Animation|Montage|MontagePlay _returnvalue "/Game/AttackCombo/AnimMontage3.AnimMontage3" 1.0 "MontageLength" 0.0 true)))))))

(fn ConstructionScript)